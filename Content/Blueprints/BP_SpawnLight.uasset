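; BP_SpawnLight is an actor that builds a row of BP_PointLight actors along X from its construction script.
; Spawn loops XUnits times, spawning each light at the running X, attaching it with relative rules, storing it in ObjectArray and advancing X by XOffset.
; Reset destroys the stored lights, clears the array and zeroes X, but no graph here calls it.
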(event EventBeginPlay)

(event Collision|EventActorBeginOverlap
  (params (OtherActor :type Actor%20Object%20Reference)))

(event EventTick
  (params (DeltaSeconds :type Float%20%28single-precision%29)))

(fn ConstructionScript
  (CallFunction|Spawn))

(fn Spawn
  (bind _output_get (Variables|Default|SetIndex (Variables|Default|GetX%20Units)))
  (while (> _output_get 0)
    (bind _returnvalue (Game|SpawnActorfromClass "/Game/Blueprints/BP_PointLight.BP_PointLight_C" (Math|Transform|MakeTransform (Math|Vector|MakeVector (Variables|Default|GetX) 0.0 0.0) "0, 0, 0" "1,1,1") "Undefined" 0 0))
    (Transformation|AttachActorToActor _returnvalue self "None" "KeepRelative" "KeepRelative" "KeepRelative" true)
    (Variables|Default|SetX (+ (Variables|Default|GetX) (Variables|Default|GetX%20Offset)))
    (Utilities|Array|Add (Variables|Default|GetObjectArray) _returnvalue)
    (Variables|Default|SetIndex (- (Variables|Default|GetIndex) 1))))

(fn Reset
  (bind _objectarray (Variables|Default|GetObjectArray))
  (for _array_element _objectarray
    (Actor|DestroyActor _array_element))
  (Utilities|Array|Clear _objectarray)
  (Variables|Default|SetX 0.0))