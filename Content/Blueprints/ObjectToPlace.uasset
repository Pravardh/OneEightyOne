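; ObjectToPlace is a placer actor that spawns BP_PointLight actors at even intervals between the first two points of its spline.
; BeginPlay caches both points' world locations and derives the interpolation step from NumberOfActors.
; GenerateAutomatically loops Alpha up to 1, spawning along a linear Ease, so placement follows a straight line rather than the curve.
; Nothing in this Blueprint calls GenerateAutomatically, and Alpha is never reset.
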(event EventBeginPlay
  (Variables|Default|SetLocation1 (.location (Spline|GetTransformatSplinePoint (Variables|Default|GetSpline) 0 "World" false)))
  (Variables|Default|SetLocation2 (.location (Spline|GetTransformatSplinePoint (Variables|Default|GetSpline) 1 "World" false)))
  (Variables|Default|SetIncrement (/ 1.0 (Variables|Default|GetNumberOfActors))))

(event Collision|EventActorBeginOverlap
  (params (OtherActor :type Actor%20Object%20Reference)))

(fn ConstructionScript)

(fn GenerateAutomatically
  (while (<= (Variables|Default|GetAlpha) 1.0)
    (Game|SpawnActorfromClass "/Game/Blueprints/BP_PointLight.BP_PointLight_C" (Math|Transform|MakeTransform (Math|Interpolation|Ease "Linear" (Variables|Default|GetAlpha) (Variables|Default|GetLocation1) (Variables|Default|GetLocation2)) "0, 0, 0" "1,1,1") "Undefined" 0 0)
    (Variables|Default|SetAlpha (+ (Variables|Default|GetAlpha) (Variables|Default|GetIncrement)))))